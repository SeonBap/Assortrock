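; BP_SnakeHead is an unfinished Blueprint, apparently for the head in a Snake game, with no working logic yet.
; Its four directional input axis events, Tick, BeginPlay, overlap event and construction script are all empty.
; Four disconnected branches hold draft movement via AddActorLocalOffset without sweep, only one scaled by delta seconds, and their comparisons have no inputs shown.
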(event EventBeginPlay)

(event Collision|EventActorBeginOverlap
  (params (OtherActor :type Actor%20Object%20Reference)))

(event EventTick
  (params (DeltaSeconds :type Float%20%28single-precision%29)))

(event Input|AxisEvents|InputAxisInput_Left
  (params (AxisValue :type Float%20%28single-precision%29)))

(event Input|AxisEvents|InputAxisInput_Right
  (params (AxisValue :type Float%20%28single-precision%29)))

(event Input|AxisEvents|InputAxisInput_Forward
  (params (AxisValue :type Float%20%28single-precision%29)))

(event Input|AxisEvents|InputAxisInput_Back
  (params (AxisValue :type Float%20%28single-precision%29)))

(fn ConstructionScript)